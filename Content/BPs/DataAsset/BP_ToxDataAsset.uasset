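; BP_ToxDataAsset builds a name-keyed dictionary of the ToxAssets found under a content path.
; LoadToxAssets clears ToxDict, then queries the Asset Registry recursively at PackagePath, including assets not yet saved to disk.
; Each result is resolved to its object, and those that cast to ToxAsset are added under their asset name.
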(event Custom|LoadToxAssets
  (Utilities|Map|Clear (Variables|Default|GetToxDict))
  (bind _outassetdata (Class|AssetRegistry|GetAssetsbyPath (Class|AssetRegistryHelpers|GetAssetRegistry) (Variables|Default|GetPackagePath) true false))
  (for _array_element _outassetdata
    (bind _astox_asset (Utilities|Casting|CastToToxAsset (Class|AssetRegistryHelpers|GetAsset _array_element)))
    (Utilities|Map|Add (Variables|Default|GetToxDict) (Utilities|String|ToString(Name) (.AssetName (Utilities|Struct|BreakAssetData _array_element))) _astox_asset)))