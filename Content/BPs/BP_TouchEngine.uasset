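; BP_TouchEngine runs a TouchDesigner TOX and shows its OUT texture on a plane through a dynamic emissive material.
; The first successful frame after loading builds a typed parameter list from the TOX's OUT_PARAMETER table, and later frames update the texture.
; SetOSCMessage filters messages by address, then loads a TOX from a catalog or sets matching parameters by style, trimming the last character from vector-style names.
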(event OnToxUnloaded(TouchEngineComponent)
  (Variables|Default|SetIsFirstReceived false))

(event OnEndFrame(TouchEngineComponent)
  (params (IsSuccessful :type Boolean) (Result :type ECookFrameResult%20Enum :default "Success") (FrameData :type Touch%20Engine%20Output%20Frame%20Data%20Structure%20%28by%20ref%29))
  (switch Utilities|FlowControl|Switch|SwitchonECookFrameResult Result
    (:Success
      (if (Variables|Default|GetIsFirstReceived)
        (bind _value (|TouchOutputK2Node (Variables|Default|GetTouchEngineComponent) "OUT"))
        (bind _output_get (Variables|Default|SetOutputTOP _value))
        (Rendering|Material|SetTextureParameterValue (Variables|Default|GetMaterial) "Tex" _output_get)
        (else
          (CallFunction|BuildCustomParameter)
          (Variables|Default|SetIsFirstReceived true))))))

(event EventBeginPlay)

(event Collision|EventActorBeginOverlap
  (params (OtherActor :type Actor%20Object%20Reference)))

(event EventTick
  (params (DeltaSeconds :type Float%20%28single-precision%29)))

(event EventEndPlay
  (params (EndPlayReason :type EEndPlayReason%20Enum :default "Destroyed"))
  (Class|TouchEngineComponentBase|StopTouchEngine (Variables|Default|GetTouchEngineComponent)))

(fn ConstructionScript
  (bind _returnvalue (Rendering|Material|CreateDynamicMaterialInstance (Variables|Default|GetPlane) 0 "/Game/Materials/M_Emissive.M_Emissive" "None" :!class /Script/Engine.PrimitiveComponent))
  (Variables|Default|SetMaterial _returnvalue))

(fn BuildCustomParameter
  (Utilities|FlowControl|Sequence
    (:then_0
      (Utilities|Array|Clear (Variables|Default|GetCustomParameters)))
    (:then_1
      (bind _value (|TouchOutputK2Node (Variables|Default|GetTouchEngineComponent) "OUT_PARAMETER"))
      (bind _index (Utilities|FlowControl|ForLoopwithBreak 0 (- (Variables|/Script/TouchEngine.TouchEngineDAT|GetNumRows _value) 1))
        (:LoopBody
          (bind _returnvalue (Class|TouchEngineDAT|GetRow _value _index))
          (bind _enum (CallFunction|ToValType (Utilities|Array|Get(acopy) _returnvalue 3)))
          (Utilities|Array|Add (Variables|Default|GetCustomParameters) (Utilities|Struct|MakeBP_CustomParameter (Utilities|Array|Get(acopy) _returnvalue) (Utilities|Array|Get(acopy) _returnvalue 1) _enum)))))))

(fn ToValType
  (params (Input :type String))
  (switch string Input
    (:Int
      (LocalVariables|SetType "NewEnumerator0"))
    (:Float
      (LocalVariables|SetType "NewEnumerator1"))
    (:Toggle
      (LocalVariables|SetType "NewEnumerator8"))
    (:Pulse
      (LocalVariables|SetType "NewEnumerator9"))
    (:Str
      (LocalVariables|SetType "NewEnumerator5"))
    (:File
      (LocalVariables|SetType "NewEnumerator7"))
    (:Menu
      (LocalVariables|SetType "NewEnumerator4"))
    (:RGB
      (LocalVariables|SetType "NewEnumerator2"))
    (:RGBA
      (LocalVariables|SetType "NewEnumerator3"))
    (:UV
      (LocalVariables|SetType "NewEnumerator6")))
  (return (LocalVariables|GetType)))

(fn SetOSCMessage
  (params (OSCMessage :type OSC%20Message%20Structure))
  (bind _returnvalue (Class|OSCManager|GetOSCMessageAddress OSCMessage))
  (bind _returnvalue_2 (Class|OSCManager|GetOSCAddressFullPath _returnvalue))
  (if (Utilities|Enum|Equal(Enum) (Variables|OSCReceive|GetAddress) (Utilities|Array|Get(acopy) (Utilities|String|ParseIntoArray _returnvalue_2 "/")))
    (Variables|Default|SetOSCMessage OSCMessage)
    (switch string (Utilities|Array|Get(acopy) (Utilities|String|ParseIntoArray _returnvalue_2 "/") 1)
      (:load
        (CallFunction|LoadTox))
      (:parameter
        (CallFunction|UpdateCustomParameters)))))

(fn UpdateCustomParameters
  (bind _returnvalue (Class|OSCManager|GetOSCMessageAddress (Variables|Default|GetOSCMessage)))
  (bind _returnvalue_2 (Class|OSCManager|GetOSCAddressFullPath _returnvalue))
  (LocalVariables|SetParamName_ (Utilities|Array|Get(acopy) (Utilities|String|ParseIntoArray _returnvalue_2 "/") 2))
  (for _array_element (Variables|Default|GetCustomParameters)
    (LocalVariables|SetName_ (.Name (Utilities|Struct|BreakBP_CustomParameter _array_element)))
    (switch Utilities|FlowControl|Switch|SwitchonENUM_VariableType (.Style (Utilities|Struct|BreakBP_CustomParameter _array_element))
      (:NewEnumerator0
        (if (Utilities|Enum|Equal(Enum) (LocalVariables|GetParamName_) (LocalVariables|GetName_)) :!label _label
          (bind _value (Class|OSCManager|GetInt32 (Variables|Default|GetOSCMessage)))
          (|TouchParameterSetK2Node (Variables|Default|GetTouchEngineComponent) (LocalVariables|GetName_) _value)
          (Development|PrintString (Utilities|String|Append "UPDATE PARAM : " (LocalVariables|GetName_)) true true "(R=0.000000,G=0.389882,B=1.000000,A=1.000000)" :!label _label_2)))
      (:NewEnumerator1
        (if (Utilities|Enum|Equal(Enum) (LocalVariables|GetParamName_) (LocalVariables|GetName_))
          (bind _value_2 (Class|OSCManager|GetFloat (Variables|Default|GetOSCMessage)))
          (|TouchParameterSetK2Node (Variables|Default|GetTouchEngineComponent) (LocalVariables|GetName_) _value_2)
          (goto _label_2)))
      (:NewEnumerator2
        (if (Utilities|Enum|Equal(Enum) (LocalVariables|GetParamName_) (Utilities|String|GetSubstring (LocalVariables|GetName_) 0 (- (Utilities|String|Len (LocalVariables|GetName_)) 1))) :!label _label_3
          (bind _values (Class|OSCManager|GetAllFloats (Variables|Default|GetOSCMessage)))
          (|TouchParameterSetK2Node (Variables|Default|GetTouchEngineComponent) (Utilities|String|GetSubstring (LocalVariables|GetName_) 0 (- (Utilities|String|Len (LocalVariables|GetName_)) 1)) _values)))
      (:NewEnumerator3
        (goto _label_3))
      (:NewEnumerator4
        (goto _label))
      (:NewEnumerator5
        (if (Utilities|Enum|Equal(Enum) (LocalVariables|GetParamName_) (LocalVariables|GetName_)) :!label _label_4
          (bind _value_3 (Class|OSCManager|GetString (Variables|Default|GetOSCMessage)))
          (|TouchParameterSetK2Node (Variables|Default|GetTouchEngineComponent) (LocalVariables|GetName_) _value_3)
          (goto _label_2)))
      (:NewEnumerator6
        (goto _label_3))
      (:NewEnumerator7
        (goto _label_4))
      (:NewEnumerator8
        (if (Utilities|Enum|Equal(Enum) (LocalVariables|GetParamName_) (LocalVariables|GetName_)) :!label _label_5
          (bind _value_4 (Class|OSCManager|GetBool (Variables|Default|GetOSCMessage)))
          (|TouchParameterSetK2Node (Variables|Default|GetTouchEngineComponent) (LocalVariables|GetName_) _value_4)
          (goto _label_2)))
      (:NewEnumerator9
        (goto _label_5)))))

(fn LoadTox
  (bind _touchenginecomponent (Variables|Default|GetTouchEngineComponent))
  (bind _value (Class|OSCManager|GetString (Variables|Default|GetOSCMessage)))
  (if (.ReturnValue (Utilities|Map|Find (Variables|/Game/BPs/DataAsset/BP_ToxDataAsset.BP_ToxDataAsset_C|GetToxDict (Variables|Default|GetToxCatalog)) _value))
    (Variables|/Script/TouchEngine.TouchEngineComponentBase|SetToxAsset _touchenginecomponent (.Value (Utilities|Map|Find (Variables|/Game/BPs/DataAsset/BP_ToxDataAsset.BP_ToxDataAsset_C|GetToxDict (Variables|Default|GetToxCatalog)) _value)))
    (Class|TouchEngineComponentBase|LoadTox _touchenginecomponent true)))